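; Kraken AI character Blueprint that supplies the enemy's health bar and floating damage-number feedback.
; On BeginPlay it binds to OnHealthChanged and pushes the current health ratio to the W_EnemyHealth widget in its HealthBarWidget.
; ShowHitNumber spawns a W_HitNumber widget at the hit location projected to screen space, registers it through StoreHitNumber and plays its animation.
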(event `self.ReceiveBeginPlay`
  (add `self.OnHealthChanged` (delegate `OnHealthChanged_Event_0`)))

(event `OnHealthChanged_Event_0` :!signature `self.OnHealthChanged`
  (params (CurHealth :type "Float (double-precision)") (MaxHealth :type "Float (double-precision)"))
  (bind _asw_enemy_health (cast `/Game/UI/Enemy/W_EnemyHealth` (`WidgetComponent.GetUserWidgetObject` (`self.HealthBarWidget`))))
  (`/Game/UI/Enemy/W_EnemyHealth.UpdateHealthBar` _asw_enemy_health (/ CurHealth MaxHealth)))

(event `self.ShowHitNumber`
  (params (Damage :type "Float (single-precision)") (HitLocation :type "Vector Structure"))
  (bind _returnvalue (`|CreateWidget` "/Game/UI/Enemy/W_HitNumber.W_HitNumber_C" null (`KismetTextLibrary.Conv_DoubleToText` Damage "HalfToEven")))
  (`UserWidget.AddToViewport` _returnvalue 0)
  (`UserWidget.SetPositionInViewport` _returnvalue (`GameplayStatics.ProjectWorldToScreen` (`GameplayStatics.GetPlayerController` 0) HitLocation) true)
  (`self.StoreHitNumber` _returnvalue HitLocation)
  (`UserWidget.PlayAnimation` _returnvalue (`/Game/UI/Enemy/W_HitNumber.HitNumberAnimation` _returnvalue) 0.0 1 "Forward" 1.0 false))

(fn `UserConstructionScript`)